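; Game mode that lets keys 1 to 4 toggle individual CP_Army actors active while held.
; BeginPlay caches every CP_Army in the level into ArmyArray, so key-to-army mapping follows the order GetAllActorsOfClass returns.
; Each key press casts the matching array element, sets its IsActive flag and prints a debug string, and release clears the flag.
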(event `self.ReceiveBeginPlay`
  (bind _outactors (`GameplayStatics.GetAllActorsOfClass` "/Game/HTOV/CP_Army.CP_Army_C"))
  (set `self.ArmyArray` _outactors))

(event `Key|One`
  (params (Key :type "Key Structure"))
  (:`Pressed`
    (bind _ascp_army (cast `/Game/HTOV/CP_Army` (`|GetArrayItem` (`self.ArmyArray`))))
    (set `/Game/HTOV/CP_Army.isActive` true _ascp_army)
    (`KismetSystemLibrary.PrintString` "Pressed 1"))
  (:`Released`
    (set `/Game/HTOV/CP_Army.isActive` false _ascp_army)))

(event `Key|Two`
  (params (Key :type "Key Structure"))
  (:`Pressed`
    (bind _ascp_army (cast `/Game/HTOV/CP_Army` (`|GetArrayItem` (`self.ArmyArray`) 1)))
    (set `/Game/HTOV/CP_Army.isActive` true _ascp_army)
    (`KismetSystemLibrary.PrintString` "Pressed 2"))
  (:`Released`
    (set `/Game/HTOV/CP_Army.isActive` false _ascp_army)))

(event `Key|Three`
  (params (Key :type "Key Structure"))
  (:`Pressed`
    (bind _ascp_army (cast `/Game/HTOV/CP_Army` (`|GetArrayItem` (`self.ArmyArray`) 2)))
    (set `/Game/HTOV/CP_Army.isActive` true _ascp_army)
    (`KismetSystemLibrary.PrintString` "Pressed 3"))
  (:`Released`
    (set `/Game/HTOV/CP_Army.isActive` false _ascp_army)))

(event `Key|Four`
  (params (Key :type "Key Structure"))
  (:`Pressed`
    (bind _ascp_army (cast `/Game/HTOV/CP_Army` (`|GetArrayItem` (`self.ArmyArray`) 3)))
    (set `/Game/HTOV/CP_Army.isActive` true _ascp_army)
    (`KismetSystemLibrary.PrintString` "Pressed 4"))
  (:`Released`
    (set `/Game/HTOV/CP_Army.isActive` false _ascp_army)))

(fn `UserConstructionScript`)